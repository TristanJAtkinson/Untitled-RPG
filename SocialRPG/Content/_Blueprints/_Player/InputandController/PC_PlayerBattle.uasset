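; Player controller for battle mode that creates and displays the battle UI.
; On BeginPlay it spawns the WB_BattleUI widget, stores a reference and adds it to the viewport.
; An event toggles mouse cursor visibility for UI interaction.
; Getter functions return this controller as the battle controller and nothing for the explore controller.
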(event `self.ReceiveBeginPlay`
  (`self.SpawnBattleUI`))

(event `SpawnBattleUI`
  (bind _returnvalue (`|CreateWidget` "/Game/GameSystems/CombatSystem/CombatWidgets/WB_BattleUI.WB_BattleUI_C"))
  (bind _output_get (set `self.REF_BattleUI` _returnvalue))
  (`UserWidget.AddToViewport` _output_get 0))

(event `SetMouseVisibilityAndInteractOptions`
  (params (`UIInput?` :type Boolean))
  (set `self.bShowMouseCursor` `UIInput?`))

(fn `GetPlayerController(Battle)`
  (returns (PlayerController :type "/Game/_Blueprints/_Player/InputandController/PC_PlayerBattle Object Reference"))
  (return self))

(fn `GetPlayerController(Explore)`
  (returns (`Player Controller` :type "/Game/_Blueprints/_Player/InputandController/PC_Player Object Reference"))
  (return null))

(fn `UserConstructionScript`)