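; BP_Player is the player character, handling movement, speed toggling on sprint input, camera flipping and world interaction.
; Enhanced Input drives movement and shifts InteractBox toward the last input, while a timeline rotates the actor's yaw for the flip.
; InteractBox stores an overlapped BPI_Interact actor for the interact key, while body overlaps send collide messages directly.
; It creates the dialogue widget, shows or removes it, and blocks movement during dialogue.
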(event `EnhancedInput|/Game/_Blueprints/_Player/InputandController/Actions/IA_Sprint`
  (params (ActionValue :type Boolean) (ElapsedSeconds :type "Float (double-precision)") (TriggeredSeconds :type "Float (double-precision)") (InputAction :type "InputAction Object Reference" :default "/Game/_Blueprints/_Player/InputandController/Actions/IA_Sprint.IA_Sprint"))
  (bind _charactermovement (`self.CharacterMovement`))
  ;[1 1 1] Sprint
  (:`Started`
    (set `CharacterMovementComponent.MaxWalkSpeed` 350.0 _charactermovement))
  (:`Canceled`
    (set `CharacterMovementComponent.MaxWalkSpeed` 600.0 _charactermovement :!label _label))
  (:`Completed`
    (goto _label)))

(event `self.ReceiveBeginPlay`
  ;[1 1 1] Add Mapping context
  (bind _aspc_player (cast `/Game/_Blueprints/_Player/InputandController/PC_Player` (`self.GetController`)))
  (`EnhancedInputSubsystemInterface.AddMappingContext` (pcsubsystem `EnhancedInputLocalPlayerSubsystem` _aspc_player) "/Game/_Blueprints/_Player/InputandController/MC_Player.MC_Player" 0 (struct))
  ;[1 1 1] Create Instance of Dialogue UI, and pass it a REF of the Player
  (bind _returnvalue (`|CreateWidget` "/Game/_Blueprints/Widgets/WB_Dialogue.WB_Dialogue_C" null self))
  (set `self.REF_DialogueWidget` _returnvalue)
  ;[1 1 1] Get REF of Player Controller
  (bind _aspc_player_2 (cast `/Game/_Blueprints/_Player/InputandController/PC_Player` (`GameplayStatics.GetPlayerController` 0)))
  (set `self.REF_PlayerController` _aspc_player_2))

(event `EnhancedInput|/Game/_Blueprints/_Player/InputandController/Actions/IA_FlipCamera`
  (params (ActionValue :type Boolean) (ElapsedSeconds :type "Float (double-precision)") (TriggeredSeconds :type "Float (double-precision)") (InputAction :type "InputAction Object Reference" :default "/Game/_Blueprints/_Player/InputandController/Actions/IA_FlipCamera.IA_FlipCamera"))
  (bind (_returnvalue_roll _returnvalue_pitch _returnvalue_yaw) (`KismetMathLibrary.BreakRotator` (`self.K2_GetActorRotation`)))
  ;[1 1 1] FlipCamera
  (:`Started`
    (`/Engine/EditorBlueprintResources/StandardMacros.FlipFlop`
      (:`A`
        (bind (_direction _fliptime) (`Timeline|FlipCamera` :!label _label_2)
          (:`Update`
            (`self.K2_SetActorRotation` (`KismetMathLibrary.MakeRotator` _returnvalue_roll _returnvalue_pitch (* _fliptime (+ _returnvalue_yaw 180.0)))))))
      (:`B`
        (goto _label_2 :!via `Reverse`)))))

(event `EnhancedInput|/Game/_Blueprints/_Player/InputandController/Actions/IA_Movement`
  (params (ActionValue :type "Vector Structure") (ElapsedSeconds :type "Float (double-precision)") (TriggeredSeconds :type "Float (double-precision)") (InputAction :type "InputAction Object Reference" :default "/Game/_Blueprints/_Player/InputandController/Actions/IA_Movement.IA_Movement"))
  (bind (_returnvalue_roll _returnvalue_pitch _returnvalue_yaw) (`KismetMathLibrary.BreakRotator` (`self.GetControlRotation`)))
  (bind (_returnvalue_roll_2 _returnvalue_pitch_2 _returnvalue_yaw_2) (`KismetMathLibrary.BreakRotator` (`self.GetControlRotation`)))
  (bind (_returnvalue_x _returnvalue_y _returnvalue_z) (`KismetMathLibrary.BreakVector` (`PawnMovementComponent.GetLastInputVector` (`self.CharacterMovement`))))
  ;[1 1 1] Movement and Interact Box relocation
  (:`Triggered`
    (if (not (`self.B_dialogueActive`))
      (`self.AddMovementInput` (`KismetMathLibrary.GetForwardVector` (`KismetMathLibrary.MakeRotator` 0.0 0.0 _returnvalue_yaw)) ActionValue_X)
      (`self.AddMovementInput` (`KismetMathLibrary.GetRightVector` (`KismetMathLibrary.MakeRotator` _returnvalue_roll_2 0.0 _returnvalue_yaw_2)) ActionValue_Y)
      (`SceneComponent.K2_SetRelativeLocation` (`self.InteractBox`) (* (`KismetMathLibrary.MakeVector` _returnvalue_x _returnvalue_y _returnvalue_z) 30.0) false false))))

(event `CameraShake`
  ;[1 1 1] Camera Shake
  (`GameplayStatics.PlayWorldCameraShake` "/Game/_Blueprints/_Player/MiscClasses/BP_CameraShake.BP_CameraShake_C" (`self.K2_GetActorLocation`) 0.0 4000.0))

(event `self.InteractBox.OnComponentBeginOverlap`
  (params (OverlappedComponent :type "PrimitiveComponent Object Reference") (OtherActor :type "Actor Object Reference") (OtherComp :type "PrimitiveComponent Object Reference") (OtherBodyIndex :type Integer) (bFromSweep :type Boolean) (SweepResult :type "HitResult Structure (by ref)"))
  ;[1 0.1804 0.8431] Detect Interactable Object
  (if (`KismetSystemLibrary.DoesImplementInterface` OtherActor "/Game/_Blueprints/_Interfaces/BPI_Interact.BPI_Interact_C")
    (set `self.A_inInteractBoxActor` OtherActor)))

(event `self.ReceiveActorBeginOverlap`
  (params (OtherActor :type "Actor Object Reference"))
  ;[1 0.1804 0.8431] Call Contact-Interaction
  (if (`KismetSystemLibrary.DoesImplementInterface` OtherActor "/Game/_Blueprints/_Interfaces/BPI_Interact.BPI_Interact_C")
    (message `/Game/_Blueprints/_Interfaces/BPI_Interact.OnCollide` OtherActor)))

(event `EnhancedInput|/Game/_Blueprints/_Player/InputandController/Actions/IA_Interact`
  (params (ActionValue :type Boolean) (ElapsedSeconds :type "Float (double-precision)") (TriggeredSeconds :type "Float (double-precision)") (InputAction :type "InputAction Object Reference" :default "/Game/_Blueprints/_Player/InputandController/Actions/IA_Interact.IA_Interact"))
  ;[1 0.1804 0.8431] Call actor in range's interact event
  (:`Started`
    (message `/Game/_Blueprints/_Interfaces/BPI_Interact.OnInteract` (`self.A_inInteractBoxActor`) (`self.REF_DialogueWidget`) self)))

(event `self.InteractBox.OnComponentEndOverlap`
  (params (OverlappedComponent :type "PrimitiveComponent Object Reference") (OtherActor :type "Actor Object Reference") (OtherComp :type "PrimitiveComponent Object Reference") (OtherBodyIndex :type Integer))
  ;[1 0.1804 0.8431] Detect Interactable Object
  (set `self.A_inInteractBoxActor` null))

(event `Dialogue Initiated`
  ;[1 0.1804 0.8431] Add / Remove Dialogue UI from viewport
  (`UserWidget.AddToViewport` (`self.REF_DialogueWidget`) 0)
  (set `self.B_dialogueActive` true))

(event `Dialogue Ended`
  ;[1 0.1804 0.8431] Add / Remove Dialogue UI from viewport
  (`Widget.RemoveFromParent` (`self.REF_DialogueWidget`))
  (set `self.B_dialogueActive` false))

(fn `UserConstructionScript`)