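; Base Blueprint class for interactable NPCs that start dialogue with the player.
; On interact, it writes its next-dialogue variable into the passed dialogue UI's current dialogue, then calls DialogueInitiated on the passed player.
; BeginPlay, overlap and Tick are disabled stubs, and the construction script only calls its parent.
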(event `/Game/_Blueprints/_Interfaces/BPI_Interact.OnInteract`
  (params (DialogueUIREF :type "/Game/_Blueprints/Widgets/WB_Dialogue Object Reference") (PlayerREF :type "/Game/_Blueprints/_Player/BP_Player Object Reference"))
  (set `/Game/_Blueprints/Widgets/WB_Dialogue.Current Dialogue` (`self.T_nextDIalogue`) DialogueUIREF)
  (`/Game/_Blueprints/_Player/BP_Player.Dialogue Initiated` PlayerREF))

(fn `UserConstructionScript`
  (`parent.UserConstructionScript`))