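; Combat game mode that sets up turn-based battles and serializes unit turns.
; On BeginPlay it blends to the battle camera, gathers party and enemy units, and fills their battle UI slots after a short delay.
; Turn requests join a unique queue; a DoOnce gate starts the front unit's turn and binds to its turn-ended dispatcher.
; GetNextTurnReady reopens the gate and starts any queued turn.
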(event `self.ReceiveBeginPlay`
  (`self.SwitchtoBattleCamera` true))

(event `SwitchtoBattleCamera`
  (params (`GoingintoBattle?` :type Boolean))
  (if `GoingintoBattle?`
    (bind _returnvalue (`GameplayStatics.GetActorOfClass` "/Game/GameSystems/CombatSystem/BP_BattleCamera.BP_BattleCamera_C"))
    (bind _output_get (set `self.REF_BattleCamera` _returnvalue))
    (`PlayerController.SetViewTargetWithBlend` (`GameplayStatics.GetPlayerController` 0) _output_get 2.5 "VTBlend_Linear" 0.0 false)
    (bind _outactors (`GameplayStatics.GetAllActorsOfClass` "/Game/GameSystems/CombatSystem/Characters/PartyUnits/BP_PartyUnitBase.BP_PartyUnitBase_C"))
    (set `self.REF_AllyUnits` _outactors)
    (bind _outactors_2 (`GameplayStatics.GetAllActorsOfClass` "/Game/GameSystems/CombatSystem/Characters/Enemies/BP_EnemyUnitBase.BP_EnemyUnitBase_C"))
    (set `self.REF_EnemyUnits` _outactors_2)
    (`KismetSystemLibrary.Delay` 0.2)
    (bind _playercontroller (message `/Game/_Blueprints/_Interfaces/BPI_Controller.GetPlayerController(Battle)` (`GameplayStatics.GetPlayerController` 0)))
    (bind _output_get_2 (set `self.REF_PlayerController` _playercontroller))
    (set `self.REF_Battle UI` (`/Game/_Blueprints/_Player/InputandController/PC_PlayerBattle.REF_BattleUI` _output_get_2))
    (for _array_element (`self.REF_AllyUnits`)
      (`/Game/GameSystems/CombatSystem/CombatWidgets/WB_BattleUI. F_AddPartySlotToUI` (`/Game/_Blueprints/_Player/InputandController/PC_PlayerBattle.REF_BattleUI` (`self.REF_PlayerController`)) _array_element))
    (for _array_element_2 (`self.REF_EnemyUnits`)
      (`/Game/GameSystems/CombatSystem/CombatWidgets/WB_BattleUI.F_AddEnemySlottoUI` (`/Game/_Blueprints/_Player/InputandController/PC_PlayerBattle.REF_BattleUI` (`self.REF_PlayerController`)) _array_element_2))))

(event `RequestNewTurn`
  (params (`Enemy Unit REF` :type "/Game/GameSystems/CombatSystem/Characters/BP_UnitBase Object Reference"))
  (`KismetArrayLibrary.Array_AddUnique` (`self.UnitTurnOrder`) `Enemy Unit REF`)
  (`self. StartNewTurn`))

(event `StartNewTurn`
  (bind _unitturnorder (`self.UnitTurnOrder`))
  (bind _bpcomp_battleoptions (`/Game/GameSystems/CombatSystem/Characters/BP_UnitBase.BPcomp_BattleOptions` (`|GetArrayItem` _unitturnorder)))
  (`/Engine/EditorBlueprintResources/StandardMacros.DoOnce` false :!label _label
    (:`Completed`
      (if (`KismetArrayLibrary.Array_IsValidIndex` _unitturnorder)
        (`/Game/GameSystems/CombatSystem/BPcomp_BattleOptions.F_StartTurnOfCurrentUnit` _bpcomp_battleoptions)
        (add `/Game/GameSystems/CombatSystem/BPcomp_BattleOptions.ED_CurrentTurnEnded` _bpcomp_battleoptions (`|CreateDelegate` :!event `GetNextTurnReady`))
        (`KismetArrayLibrary.Array_Remove` (`self.UnitTurnOrder`))
        (else
          (`self.GetNextTurnReady`))))))

(event `GetNextTurnReady`
  (`|ExecutionSequence`
    (:`then_0`
      (goto _label :!via `Reset`))
    (:`then_1`
      (if (`KismetArrayLibrary.Array_IsValidIndex` (`self.UnitTurnOrder`))
        (`self. StartNewTurn`)))))

(fn `GetGamemodeCombatREF`
  (returns (GamemodeREF :type "/Game/GameSystems/Gamemodes/GM_Combat Object Reference"))
  (return self))

(fn `UserConstructionScript`)