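; Turn-based battle camera actor on a spring arm that snaps to a unit and can orbit it.
; SetOrbit, switched on at BeginPlay, toggles the RotatingMovement spin and spring arm yaw inheritance, resetting actor rotation when off.
; SetCameraLocation attaches to the given actor; its fallback location branch only reassigns the value to itself.
; Tick's interpolation while attached targets the current location, adding no movement.
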(event `self.ReceiveTick`
  (params (DeltaSeconds :type "Float (single-precision)"))
  (`/Engine/EditorBlueprintResources/StandardMacros.IsValid` (`self.GetAttachParentActor`)
    (:`Is Valid`
      (`self.K2_SetActorLocation` (`KismetMathLibrary.VInterpTo` (`self.K2_GetActorLocation`) (`self.K2_GetActorLocation`) (`GameplayStatics.GetWorldDeltaSeconds`) (`self.F_InterpSpeed`))))))

(event `self.ReceiveBeginPlay`
  (`self.SetOrbit` true))

(event `/Game/_Blueprints/_Interfaces/BPI_BatleCamera.SetOrbit`
  (params (` IsOrbitingCamera` :type Boolean))
  ;[1 1 1] Set Orbit rate of the Camera if orbiting, called from --
  (set `RotatingMovementComponent.RotationRate` (`KismetMathLibrary.SelectRotator` (struct :`Yaw` 11.0) (struct) ` IsOrbitingCamera`) (`self.RotatingMovement`))
  (bind _output_get (set `SpringArmComponent.bInheritYaw` ` IsOrbitingCamera` (`self.SpringArm`)))
  (if (not _output_get)
    (`self.K2_SetActorRotation` (struct))))

(event `/Game/_Blueprints/_Interfaces/BPI_BatleCamera.SetCameraLocation`
  (params (`Actor REF` :type "Actor Object Reference") (CameraDesiredLoc :type "Vector Structure"))
  ;[1 1 1] Attatches Actor to parent unit character whose turn it is, or a desired vector location if actor REF isn't valid
  (`/Engine/EditorBlueprintResources/StandardMacros.IsValid` `Actor REF`
    (:`Is Valid`
      (`self.K2_AttachToActor` `Actor REF` "None" "SnapToTarget" "SnapToTarget" "SnapToTarget")
      (`SceneComponent.K2_SetRelativeRotation` :`self` (`self.Camera`)))
    (:`Is Not Valid`
      (set `self.Camera Desired Loc` CameraDesiredLoc))))

(fn `UserConstructionScript`)